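; BPC_Damageable is a health component that tracks damage and healing for its owner.
; CurrentHealth starts at MaxHealth on BeginPlay, then ReceiveDamage subtracts from it and ReceiveHeal adds to it.
; Reaching zero or below only prints "Dead!", and neither function clamps the health value.
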(event `self.ReceiveBeginPlay`
  (set `self.CurrentHealth` (`self.MaxHealth`)))

(fn `ReceiveDamage`
  (params (NewParam :type "Float (double-precision)"))
  (bind _output_get (set `self.CurrentHealth` (- (`self.CurrentHealth`) NewParam)))
  (if (<= _output_get 0.0)
    (`KismetSystemLibrary.PrintString` "Dead!"))
  (return))

(fn `ReceiveHeal`
  (params (HealAmount :type "Float (double-precision)"))
  (set `self.CurrentHealth` (+ (`self.CurrentHealth`) HealAmount)))